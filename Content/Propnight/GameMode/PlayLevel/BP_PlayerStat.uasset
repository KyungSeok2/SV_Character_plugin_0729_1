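; BP_PlayerStat is a player stat Blueprint that holds health and handles damage and death notification.
; AddDamage subtracts from HP within a fixed clamp, prints debug text, and calls the death dispatcher when HP reaches zero.
; HP's RepNotify broadcasts the HP dispatcher, passing MaxHP as zero rather than a real maximum.
; The construction script is empty, and a node clearing the Death flag is left unconnected.
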(fn ConstructionScript)

(fn OnRepHP
  (Default|CallEventDispatcherHP (Variables|Default|GetHP) 0.0))

(fn AddDamage
  (params (Damage :type Float%20%28single-precision%29))
  (bind _output_get (Variables|Default|SetHP (Math|Float|Clamp(Float) (- (Variables|Default|GetHP) Damage) 0.0 1e+02)))
  (Development|PrintString (Utilities|String|Append (Utilities|String|ToString(Float) Damage) "Damage"))
  (if (<= _output_get 0.0)
    (Development|PrintString "Die")
    (Default|CallEventDispatcherDeath)))